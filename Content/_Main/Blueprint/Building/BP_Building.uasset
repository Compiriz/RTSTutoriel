(event `self.Cube.OnComponentBeginOverlap`
  (params (OverlappedComponent :type "PrimitiveComponent Object Reference") (OtherActor :type "Actor Object Reference") (OtherComp :type "PrimitiveComponent Object Reference") (OtherBodyIndex :type Integer) (bFromSweep :type Boolean) (SweepResult :type "HitResult Structure (by ref)"))
  (if (not (`self.bConstructed`))
    (`PrimitiveComponent.SetMaterial` (`self.Cube`) 0 "/Game/_Main/Material/Building/ValidConstruction/M_NotValid.M_NotValid")))

(event `self.Cube.OnComponentEndOverlap`
  (params (OverlappedComponent :type "PrimitiveComponent Object Reference") (OtherActor :type "Actor Object Reference") (OtherComp :type "PrimitiveComponent Object Reference") (OtherBodyIndex :type Integer))
  (if (not (`self.bConstructed`))
    (`PrimitiveComponent.SetMaterial` (`self.Cube`) 0 "/Game/_Main/Material/Building/ValidConstruction/M_Valid.M_Valid")))

(fn `Attacked`
  (params (NewAggressor :type "/Game/_Main/Blueprint/Unit/BP_Unit Object Reference") (Damage :type Integer))
  (returns (bIsDetroyed :type Boolean))
  (bind _output_get (set `self.Life` (- (`self.Life`) 10)))
  (if (<= _output_get 0)
    (`self.K2_DestroyActor`)
    (return true)
    (else
      (return false))))

(fn `Build`
  (returns (Built :type Boolean))
  (bind _cube (`self.Cube`))
  (if (`KismetArrayLibrary.Array_IsEmpty` (`self.GetOverlappingActors` "/Script/Engine.Actor"))
    (`PrimitiveComponent.SetCollisionProfileName` _cube "BuildingCollision" true)
    (`PrimitiveComponent.SetMaterial` _cube 0 "/Game/_Main/Material/Building/ValidConstruction/M_Constructed.M_Constructed")
    (set `self.bConstructed` true)
    (return true)
    (else
      (`PrimitiveComponent.SetMaterial` _cube 0 "/Game/_Main/Material/Building/ValidConstruction/M_NotValid.M_NotValid")
      (return false))))

(fn `GetTeamIndex`
  (returns (TeamIndex :type Byte))
  (return (`self.TeamIndex`)))

(fn `UserConstructionScript`)