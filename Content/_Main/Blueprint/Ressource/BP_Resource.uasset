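; BP_Resource is a resource actor that holds a typed Quantity to be extracted.
; Its Extraction function subtracts the given power from Quantity while it is positive, returning the type and that full power as collected, even beyond what remains.
; Once Quantity is depleted, a later non-zero extraction destroys the actor and returns the leftover Quantity, which can be zero or negative.
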(fn `Extraction`
  (params (ExtractionPower :type Integer))
  (returns (Type :type "/Game/_Main/Blueprint/Ressource/E_RessourceType Enum") (Collected :type Integer))
  (if (< 0.0 (`self.Quantity`))
    (set `self.Quantity` (- (`self.Quantity`) (`local.ExtractionPower`)))
    (return (`self.Type`) (`local.ExtractionPower`))
    (elif (!= ExtractionPower 0)
      (`self.K2_DestroyActor`)
      (return (`self.Type`) (`self.Quantity`)))))

(fn `UserConstructionScript`)