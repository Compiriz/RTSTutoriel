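; BP_Unit is a team-based combat unit with life, a selection focus indicator and cooldown-gated attacks.
; It resolves its owning BP_Player by matching team index across player controllers.
; Attacks go through interface messages; a hit unit passes the aggressor to its controller as target, loses life and is destroyed at zero.
; On capsule hits, it nudges stationary, targetless teammates along its forward vector.
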(event `self.ReceiveBeginPlay`
  (set `self.Player` (`|ConvertAsset` (`self.GetPlayer`))))

(event `/Game/_Main/Blueprint/Interface/BPI_Selectable.Attacked`
  (params (Aggressor :type "/Game/_Main/Blueprint/Unit/BP_Unit Object Reference") (Damage :type Integer))
  (`/Engine/EditorBlueprintResources/StandardMacros.IsValid` (`self.Aggressor`)
    (:`Is Valid`
      _)
    (:`Is Not Valid`
      (bind _output_get (set `self.Aggressor` Aggressor))))
  (message `/Game/_Main/Blueprint/Unit/AIController/Interface/BPI_UnitController.SetTarget` (`self.GetController`) _output_get)
  (bind _output_get_2 (set `self.Life` (- (`self.Life`) Damage)))
  (if (<= _output_get_2 0)
    (`self.K2_DestroyActor`)))

(event `self.CapsuleComponent.OnComponentHit`
  (params (HitComponent :type "PrimitiveComponent Object Reference") (OtherActor :type "Actor Object Reference") (OtherComp :type "PrimitiveComponent Object Reference") (NormalImpulse :type "Vector Structure") (Hit :type "HitResult Structure (by ref)"))
  (if (`KismetSystemLibrary.DoesImplementInterface` OtherActor)
    (`KismetSystemLibrary.DelayUntilNextTick`)
    (bind _teamindex (message `/Game/_Main/Blueprint/Interface/BPI_Selectable.GetTeamIndex` OtherActor))
    (bind _target (message `/Game/_Main/Blueprint/Unit/AIController/Interface/BPI_UnitController.GetTarget` (`AIBlueprintHelperLibrary.GetAIController` OtherActor)))
    (if (and (== _teamindex (`self.TeamIndex`)) (not (`KismetSystemLibrary.IsValid` _target)) (== (`self.GetVelocity` OtherActor) (0.0 0.0 0.0)))
      (`self.K2_AddActorWorldOffset` OtherActor (* (`self.GetActorForwardVector`) 20.0) true false))))

(fn `Action`
  (params (SelectedTarget :type "Object Object Reference"))
  (if (`self.VerifyCooldown`)
    (`self.ResetCooldown`)
    (message `/Game/_Main/Blueprint/Interface/BPI_Selectable.Attacked` (`local.SelectedTarget`) self (`self.Damage`))))

(fn `GetPlayer`
  (returns (ReturnValue :type "/Game/_Main/Blueprint/Player/BP_Player Object Reference"))
  (locals (PlayerToOutput :type "/Game/_Main/Blueprint/PlayerController/BP_PlayerController Object Reference"))
  (bind _outactors (`GameplayStatics.GetAllActorsOfClass` "/Game/_Main/Blueprint/PlayerController/BP_PlayerController.BP_PlayerController_C"))
  (for _array_element _outactors
    (if (== (`/Game/_Main/Blueprint/PlayerController/BP_PlayerController.TeamIndex` _array_element) (`self.TeamIndex`))
      (set `local.PlayerToOutput` _array_element)
      (break)))
  (bind _asbp_player (cast `/Game/_Main/Blueprint/Player/BP_Player` (`Controller.K2_GetPawn` (`local.PlayerToOutput`))))
  (return _asbp_player))

(fn `GetTeamIndex`
  (returns (TeamIndex :type Byte))
  (return (`self.TeamIndex`)))

(fn `ResetCooldown`
  (set `self.LastTime` (`GameplayStatics.GetTimeSeconds`)))

(fn `ToggleFocus`
  (params (bNewVisibility :type Boolean))
  (`SceneComponent.SetVisibility` (`self.Focus`) bNewVisibility false))

(fn `UserConstructionScript`)

(fn `VerifyCooldown`
  (returns (ReturnValue :type Boolean))
  (return (< (`self.Cooldown`) (- (`GameplayStatics.GetTimeSeconds`) (`self.LastTime`)))))