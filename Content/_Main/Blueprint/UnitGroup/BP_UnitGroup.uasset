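; BP_UnitGroup is an actor that represents a group of units, stored as an array of their AI controllers.
; CreateArmy spawns infantry, anti-cavalry, archery or cavalry by Type in a two-wide grid at its location, registering each controller with the group.
; BeginPlay flags the group as military if any existing member is not a Harvest unit.
; FocusAll turns on focus for every member pawn, and GetGroup exposes the array and military flag.
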(event `self.ReceiveBeginPlay`
  (for _array_element (`self.Group`)
    (if (`|EnumInequality` (`/Game/_Main/Blueprint/Unit/BP_Unit.Type` (`/Game/_Main/Blueprint/Unit/AIController/AIC_Unit.ControlledPawn` _array_element)) "NewEnumerator5")
      (set `self.Is Military Army` true)
      (break))))

(event `/Game/_Main/Blueprint/UnitGroup/BPI_UnitGroup.FocusAll`
  (params (bTrue :type Boolean))
  (for _array_element (`self.Group`)
    (`/Game/_Main/Blueprint/Unit/BP_Unit.ToggleFocus` (`/Game/_Main/Blueprint/Unit/AIController/AIC_Unit.ControlledPawn` _array_element) bTrue)))

(fn `CreateArmy`
  (for _index (range 1 (+ (`self.Count`) 1))
    (switch `/Game/_Main/Blueprint/Unit/E_UnitType` (`self.Type`)
      (:`NewEnumerator1`
        (bind _returnvalue (`KismetMathLibrary.MakeTransform` (+ (`KismetMathLibrary.MakeVector` (`KismetMathLibrary.Conv_IntToDouble` (* (/ _index 2) 150)) (`KismetMathLibrary.Conv_IntToDouble` (* (mod _index 2) 150))) (`self.K2_GetActorLocation`))))
        (bind _returnvalue_2 (`|SpawnActorFromClass` "/Game/_Main/Blueprint/UnitType/Infantry/BP_Infantry.BP_Infantry_C" _returnvalue "Undefined" "MultiplyWithRoot" null null))
        (bind _returnvalue_3 (`AIBlueprintHelperLibrary.GetAIController` _returnvalue_2))
        (`KismetArrayLibrary.Array_Add` (`self.Group`) _returnvalue_3)
        (message `/Game/_Main/Blueprint/Unit/AIController/Interface/BPI_UnitController.SetUnitGroup` _returnvalue_3 self))
      (:`NewEnumerator2`
        (bind _returnvalue_4 (`|SpawnActorFromClass` "/Game/_Main/Blueprint/UnitType/Anti-Calvary/BP_Anti-Calvary.BP_Anti-Calvary_C" _returnvalue "Undefined" "MultiplyWithRoot" null null))
        (bind _returnvalue_5 (`AIBlueprintHelperLibrary.GetAIController` _returnvalue_4))
        (`KismetArrayLibrary.Array_Add` (`self.Group`) _returnvalue_5)
        (message `/Game/_Main/Blueprint/Unit/AIController/Interface/BPI_UnitController.SetUnitGroup` _returnvalue_5 self))
      (:`NewEnumerator3`
        (bind _returnvalue_6 (`|SpawnActorFromClass` "/Game/_Main/Blueprint/UnitType/Archery/BP_Archery.BP_Archery_C" _returnvalue "Undefined" "MultiplyWithRoot" null null))
        (bind _returnvalue_7 (`AIBlueprintHelperLibrary.GetAIController` _returnvalue_6))
        (`KismetArrayLibrary.Array_Add` (`self.Group`) _returnvalue_7)
        (message `/Game/_Main/Blueprint/Unit/AIController/Interface/BPI_UnitController.SetUnitGroup` _returnvalue_7 self))
      (:`NewEnumerator4`
        (bind _returnvalue_8 (`|SpawnActorFromClass` "/Game/_Main/Blueprint/UnitType/Calvary/BP_Calvary.BP_Calvary_C" _returnvalue "Undefined" "MultiplyWithRoot" null null))
        (bind _returnvalue_9 (`AIBlueprintHelperLibrary.GetAIController` _returnvalue_8))
        (`KismetArrayLibrary.Array_Add` (`self.Group`) _returnvalue_9)
        (message `/Game/_Main/Blueprint/Unit/AIController/Interface/BPI_UnitController.SetUnitGroup` _returnvalue_9 self)))))

(fn `GetGroup`
  (returns (Group :type "Array of AIController Object Reference") (bIsMilitaryArmy :type Boolean))
  (return (`self.Group`) (`self.Is Military Army`)))

(fn `UserConstructionScript`)