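; RTS player controller for camera movement, unit selection and grouping, orders, and building placement.
; Click or HUD-drawn drag box fills the Army array; orders resolve as gather, attack, or grid-formation move through interface messages.
; Looping timers drive hover highlighting and the cursor-following building preview, with optional grid snapping.
; Input mapping contexts switch between select, order and building modes, while a MoreOption modifier alters selection, rotation, grouping and repeat construction.
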(event `self.ReceiveBeginPlay`
  (bind _returnvalue (subsystem `EnhancedInputLocalPlayerSubsystem`))
  (bind _asbp_hud (cast `/Game/_Main/Blueprint/HUD/BP_HUD` (`self.GetHUD`)))
  (set `self.HUD` _asbp_hud)
  (`EnhancedInputSubsystemInterface.AddMappingContext` _returnvalue "/Game/_Main/Blueprint/PlayerController/Input/IMC/Default/IMC_Default.IMC_Default" 0 (struct))
  (`EnhancedInputSubsystemInterface.AddMappingContext` _returnvalue "/Game/_Main/Blueprint/PlayerController/Input/IMC/Select/IMC_Select.IMC_Select" 0 (struct))
  (bind _returnvalue_2 (`KismetSystemLibrary.K2_SetTimer` null "HoverUnit" 0.03 true))
  (set `self.HoverUnitTimer` _returnvalue_2))

(event `EnhancedInput|/Game/_Main/Blueprint/PlayerController/Input/Input/Building/IA_BuildingConstruct`
  (params (ActionValue :type Boolean) (ElapsedSeconds :type "Float (double-precision)") (TriggeredSeconds :type "Float (double-precision)") (InputAction :type "InputAction Object Reference" :default "/Game/_Main/Blueprint/PlayerController/Input/Input/Building/IA_BuildingConstruct.IA_BuildingConstruct"))
  (:`Completed`
    (`self.BuildBuilding`)))

(event `EnhancedInput|/Game/_Main/Blueprint/PlayerController/Input/Input/Default/IA_MoreOption`
  (params (ActionValue :type Boolean) (ElapsedSeconds :type "Float (double-precision)") (TriggeredSeconds :type "Float (double-precision)") (InputAction :type "InputAction Object Reference" :default "/Game/_Main/Blueprint/PlayerController/Input/Input/Default/IA_MoreOption.IA_MoreOption"))
  (:`Started`
    (set `self.bMoreOption` true))
  (:`Completed`
    (set `self.bMoreOption` false)))

(event `EnhancedInput|/Game/_Main/Blueprint/PlayerController/Input/Input/Default/IA_Move`
  (params (ActionValue :type "Vector2D Structure") (ElapsedSeconds :type "Float (double-precision)") (TriggeredSeconds :type "Float (double-precision)") (InputAction :type "InputAction Object Reference" :default "/Game/_Main/Blueprint/PlayerController/Input/Input/Default/IA_Move.IA_Move"))
  (:`Triggered`
    (`self.PlayerMovement` ActionValue_X ActionValue_Y)))

(event `EnhancedInput|/Game/_Main/Blueprint/PlayerController/Input/Input/Default/IA_Zoom`
  (params (ActionValue :type "Float (double-precision)") (ElapsedSeconds :type "Float (double-precision)") (TriggeredSeconds :type "Float (double-precision)") (InputAction :type "InputAction Object Reference" :default "/Game/_Main/Blueprint/PlayerController/Input/Input/Default/IA_Zoom.IA_Zoom"))
  (:`Triggered`
    (`self.ZoomCamera` ActionValue)))

(event `EnhancedInput|/Game/_Main/Blueprint/PlayerController/Input/Input/Default/IA_Rotate`
  (params (ActionValue :type "Float (double-precision)") (ElapsedSeconds :type "Float (double-precision)") (TriggeredSeconds :type "Float (double-precision)") (InputAction :type "InputAction Object Reference" :default "/Game/_Main/Blueprint/PlayerController/Input/Input/Default/IA_Rotate.IA_Rotate"))
  ; Rotate
  (:`Triggered`
    (`self.K2_AddActorLocalRotation` (`GameplayStatics.GetPlayerPawn` 0) (`KismetMathLibrary.MakeRotator` 0.0 0.0 ActionValue) false false)))

(event `EnhancedInput|/Game/_Main/Blueprint/PlayerController/Input/Input/Order/IA_GiveOrder`
  (params (ActionValue :type Boolean) (ElapsedSeconds :type "Float (double-precision)") (TriggeredSeconds :type "Float (double-precision)") (InputAction :type "InputAction Object Reference" :default "/Game/_Main/Blueprint/PlayerController/Input/Input/Order/IA_GiveOrder.IA_GiveOrder"))
  (:`Completed`
    (bind _bissuccessful (`self.RessourceOnClick`))
    (if (not _bissuccessful)
      (bind _bissuccessful_2 (`self.AttackEnemy`))
      (if (not _bissuccessful_2)
        (`self.GiveUnitLocation`)))))

(event `EnhancedInput|/Game/_Main/Blueprint/PlayerController/Input/Input/Building/IA_PrecisionConstruct`
  (params (ActionValue :type Boolean) (ElapsedSeconds :type "Float (double-precision)") (TriggeredSeconds :type "Float (double-precision)") (InputAction :type "InputAction Object Reference" :default "/Game/_Main/Blueprint/PlayerController/Input/Input/Building/IA_PrecisionConstruct.IA_PrecisionConstruct"))
  (:`Started`
    (if (`self.bPrecisionBuilding`)
      (set `self.bPrecisionBuilding` false)
      (else
        (set `self.bPrecisionBuilding` true)))))

(event `EnhancedInput|/Game/_Main/Blueprint/PlayerController/Input/Input/Select/IA_Click`
  (params (ActionValue :type Boolean) (ElapsedSeconds :type "Float (double-precision)") (TriggeredSeconds :type "Float (double-precision)") (InputAction :type "InputAction Object Reference" :default "/Game/_Main/Blueprint/PlayerController/Input/Input/Select/IA_Click.IA_Click"))
  (:`Triggered`
    (`self.UpdateMousePositionDrawRect`))
  (:`Started`
    (`self.StartDrawRect`))
  (:`Completed`
    (`self.StopDrawRect`)
    (if (`self.bHasArmy`)
      (set `self.bHasArmy` false)
      (else
        (bind _hasnotselectedunit (`self.SelectUnitOnClick`))
        (if _hasnotselectedunit
          (`self.SelectBuildingOnClick`))))))

(event `EnhancedInput|/Game/_Main/Blueprint/PlayerController/Input/Input/Building/IA_RotateBuilding`
  (params (ActionValue :type Boolean) (ElapsedSeconds :type "Float (double-precision)") (TriggeredSeconds :type "Float (double-precision)") (InputAction :type "InputAction Object Reference" :default "/Game/_Main/Blueprint/PlayerController/Input/Input/Building/IA_RotateBuilding.IA_RotateBuilding"))
  (bind _buildingpreview (`self.BuildingPreview`))
  (:`Started`
    (if (`self.bMoreOption`)
      (`self.K2_AddActorWorldRotation` _buildingpreview (struct :`Yaw` 25.0) false false)
      (else
        (`self.K2_AddActorWorldRotation` _buildingpreview (struct :`Yaw` -25.0) false false)))))

(event `EnhancedInput|/Game/_Main/Blueprint/PlayerController/Input/Input/Order/IA_MakeGroup`
  (params (ActionValue :type Boolean) (ElapsedSeconds :type "Float (double-precision)") (TriggeredSeconds :type "Float (double-precision)") (InputAction :type "InputAction Object Reference" :default "/Game/_Main/Blueprint/PlayerController/Input/Input/Order/IA_MakeGroup.IA_MakeGroup"))
  (:`Started`
    (`self.CreateGroup`)))

(fn `AddUnitsToArmy`
  (params (Array :type "Array of Actor Object Reference"))
  (for _array_element Array
    (bind _selectedunit (message `/Game/_Main/Blueprint/Unit/AIController/Interface/BPI_UnitController.Selected` (`AIBlueprintHelperLibrary.GetAIController` _array_element)))
    (`KismetArrayLibrary.Array_AddUnique` (`self.Army`) _selectedunit))
  (`EnhancedInputSubsystemInterface.AddMappingContext` (subsystem `EnhancedInputLocalPlayerSubsystem`) "/Game/_Main/Blueprint/PlayerController/Input/IMC/Order/IMC_Order.IMC_Order" 0 (struct))
  (set `self.bHasArmy` true))

(fn `AttackEnemy`
  (returns (bIsSuccessful :type Boolean))
  (bind (_returnvalue _hitactor) (`self.GetActorFromHit` (`|MakeArray` "ObjectTypeQuery7" "ObjectTypeQuery8" :!type "EObjectTypeQuery Enum")))
  (bind _teamindex (message `/Game/_Main/Blueprint/Interface/BPI_Selectable.GetTeamIndex` _hitactor))
  (if (!= _teamindex (`self.TeamIndex`))
    (`self.SetTargetToUnitInArmy` _hitactor)
    (return true)))

(fn `BuildBuilding`
  (bind _returnvalue (subsystem `EnhancedInputLocalPlayerSubsystem`))
  (bind _bcanbuild (message `/Game/_Main/Blueprint/Building/Interface/BPI_Building.Build` (`self.BuildingPreview`)))
  (if _bcanbuild
    (if (`self.bMoreOption`)
      (`self.CreateBuildingPreview` (`GameplayStatics.GetObjectClass` (`self.BuildingPreview`)))
      (else
        (`KismetSystemLibrary.K2_ClearAndInvalidateTimerHandle` (`self.BuildingPositionTimer`))
        (`EnhancedInputSubsystemInterface.AddMappingContext` _returnvalue "/Game/_Main/Blueprint/PlayerController/Input/IMC/Select/IMC_Select.IMC_Select" 0 (struct))
        (`EnhancedInputSubsystemInterface.RemoveMappingContext` _returnvalue "/Game/_Main/Blueprint/PlayerController/Input/IMC/Building/IMC_Building.IMC_Building" (struct))
        (set `self.BuildingPreview` null)
        (`KismetSystemLibrary.K2_UnPauseTimerHandle` (`self.HoverUnitTimer`))))))

(fn `BuildingPosition`
  (bind _buildingpreview (`self.BuildingPreview`))
  (bind _buildingpreview_2 (`self.BuildingPreview`))
  (bind (_bblockinghit _binitialoverlap _time _distance _location _impactpoint) (`GameplayStatics.BreakHitResult` (`self.GetHitResultUnderCursorForObjects` (`|MakeArray` "ObjectTypeQuery1" :!type "EObjectTypeQuery Enum"))))
  (bind (_returnvalue_x _returnvalue_y) (`KismetMathLibrary.BreakVector` (/ _impactpoint 100.0)))
  (if (== _impactpoint (0.0 0.0 0.0))
    (`self.SetActorHiddenInGame` _buildingpreview true)
    (else
      (`self.SetActorHiddenInGame` _buildingpreview false)
      (if (`self.bPrecisionBuilding`)
        (`self.K2_SetActorLocation` _buildingpreview_2 (`KismetMathLibrary.MakeVector` (* (`KismetMathLibrary.Round` _returnvalue_x) 100.0) (* (`KismetMathLibrary.Round` _returnvalue_y) 100.0)) false false)
        (else
          (`self.K2_SetActorLocation` _buildingpreview_2 _impactpoint false false))))))

(fn `ChangeArmyFromRectSelection`
  (params (bisMilitaryArmy :type Boolean) (NewArmy :type "Array of Actor Object Reference (by ref)"))
  (if (`KismetArrayLibrary.Array_IsEmpty` NewArmy)
    (if (`self.bMoreOption`)
      (set `self.bHasArmy` false)
      (else
        (`self.ResetArmy`)))
    (else
      (set `self.Is Military Army` bisMilitaryArmy)
      (bind _bisreset (`self.DeselectArmy`))
      (if _bisreset
        (`KismetArrayLibrary.Array_Clear` (`self.Army`)))
      (`self.AddUnitsToArmy` (`local.NewArmy`)))))

(fn `CreateBuildingPreview`
  (params (BuildingClass :type "/Game/_Main/Blueprint/Building/BP_Building Class Reference") (bIsNotMultipleConstruct :type Boolean))
  (bind _returnvalue (subsystem `EnhancedInputLocalPlayerSubsystem`))
  (bind _hoverunittimer (`self.HoverUnitTimer`))
  (for _array_element (`self.Army`)
    (message `/Game/_Main/Blueprint/Unit/AIController/Interface/BPI_UnitController.Deselected` _array_element))
  (`KismetArrayLibrary.Array_Clear` (`self.Army`))
  (`/Game/_Main/Blueprint/Unit/BP_Unit.ToggleFocus` (`self.Focused`) false)
  (`EnhancedInputSubsystemInterface.RemoveMappingContext` (subsystem `EnhancedInputLocalPlayerSubsystem`) "/Game/_Main/Blueprint/PlayerController/Input/IMC/Order/IMC_Order.IMC_Order" (struct))
  (if (`local.bIsNotMultipleConstruct`)
    (`/Engine/EditorBlueprintResources/StandardMacros.IsValid` (`self.BuildingPreview`)
      (:`Is Valid`
        (`KismetSystemLibrary.K2_UnPauseTimerHandle` _hoverunittimer)
        (`EnhancedInputSubsystemInterface.AddMappingContext` _returnvalue "/Game/_Main/Blueprint/PlayerController/Input/IMC/Select/IMC_Select.IMC_Select" 0 (struct))
        (`EnhancedInputSubsystemInterface.RemoveMappingContext` _returnvalue "/Game/_Main/Blueprint/PlayerController/Input/IMC/Building/IMC_Building.IMC_Building" (struct))
        (`self.K2_DestroyActor` (`self.BuildingPreview`))
        (`KismetSystemLibrary.K2_ClearAndInvalidateTimerHandle` (`self.BuildingPositionTimer`))
        (set `self.BuildingPreview` null))
      (:`Is Not Valid`
        (`KismetSystemLibrary.K2_PauseTimerHandle` _hoverunittimer :!label _label)
        (`EnhancedInputSubsystemInterface.AddMappingContext` _returnvalue "/Game/_Main/Blueprint/PlayerController/Input/IMC/Building/IMC_Building.IMC_Building" 0 (struct))
        (`EnhancedInputSubsystemInterface.RemoveMappingContext` _returnvalue "/Game/_Main/Blueprint/PlayerController/Input/IMC/Select/IMC_Select.IMC_Select" (struct))
        (bind _returnvalue_2 (`|SpawnActorFromClass` (`local.BuildingClass`) (`KismetMathLibrary.MakeTransform` (0.0 0.0 -500.0)) "Undefined" "MultiplyWithRoot" null null))
        (set `self.BuildingPreview` _returnvalue_2)
        (bind _returnvalue_3 (`KismetSystemLibrary.K2_SetTimer` null "BuildingPosition" 0.02 true))
        (set `self.BuildingPositionTimer` _returnvalue_3)))
    (else
      (goto _label))))

(fn `CreateGroup`
  (if (`self.bMoreOption`)
    (for _array_element (`self.Army`)
      (bind _unitgroup (message `/Game/_Main/Blueprint/Unit/AIController/Interface/BPI_UnitController.GetUnitGroup` _array_element))
      (`/Engine/EditorBlueprintResources/StandardMacros.IsValid` _unitgroup
        (:`Is Valid`
          (`self.K2_DestroyActor` _unitgroup))))
    (else
      (bind _returnvalue (`|SpawnActorFromClass` "/Game/_Main/Blueprint/UnitGroup/BP_UnitGroup.BP_UnitGroup_C" (`KismetMathLibrary.MakeTransform` (0.0 0.0 0.0)) "Undefined" "MultiplyWithRoot" null (`self.Army`) 0 "NewEnumerator0" null))
      (for _array_element_2 (`self.Army`)
        (bind _unitgroup_2 (message `/Game/_Main/Blueprint/Unit/AIController/Interface/BPI_UnitController.GetUnitGroup` _array_element_2))
        (`/Engine/EditorBlueprintResources/StandardMacros.IsValid` _unitgroup_2
          (:`Is Valid`
            (`self.K2_DestroyActor` _unitgroup_2))
          (:`Is Not Valid`
            _))
        (message `/Game/_Main/Blueprint/Unit/AIController/Interface/BPI_UnitController.SetUnitGroup` _array_element_2 _returnvalue)))))

(fn `DeselectArmy`
  (returns (bIsReset :type Boolean))
  (if (`self.bMoreOption`)
    (return false)
    (else
      (for _array_element (`self.Army`)
        (message `/Game/_Main/Blueprint/Unit/AIController/Interface/BPI_UnitController.Deselected` _array_element))
      (return true))))

(fn `GetActorFromHit`
  (params (ObjectTypes :type "Array of EObjectTypeQuery Enum (by ref)"))
  (returns (ReturnValue :type Boolean) (HitActor :type "Actor Object Reference") (HitResult :type "HitResult Structure"))
  (bind (_hitresult _returnvalue) (`self.GetHitResultUnderCursorForObjects` ObjectTypes false))
  (return _returnvalue (`.HitActor` (`GameplayStatics.BreakHitResult` _hitresult)) _hitresult))

(fn `GiveUnitLocation`
  (for (_array_element _array_index) (`self.Army`)
    (message `/Game/_Main/Blueprint/Unit/AIController/Interface/BPI_UnitController.CancelAction` _array_element true)
    (message `/Game/_Main/Blueprint/Unit/AIController/Interface/BPI_UnitController.SetTarget` _array_element null)
    (message `/Game/_Main/Blueprint/Unit/AIController/Interface/BPI_UnitController.MoveTo` _array_element (+ (`KismetMathLibrary.MakeVector` (`KismetMathLibrary.Conv_IntToDouble` (* (/ _array_index 2) 150)) (`KismetMathLibrary.Conv_IntToDouble` (* (mod _array_index 2) 150))) (`.Location` (`GameplayStatics.BreakHitResult` (`self.GetHitResultUnderCursorByChannel` "TraceTypeQuery1")))))))

(fn `HoverUnit`
  (locals (HoveredUnit :type "/Game/_Main/Blueprint/Unit/BP_Unit Object Reference"))
  (bind (_returnvalue _hitactor) (`self.GetActorFromHit` (`|MakeArray` (cast `EObjectTypeQuery` 6))))
  (if _returnvalue
    (bind _asbp_unit (cast `/Game/_Main/Blueprint/Unit/BP_Unit` _hitactor))
    (set `local.HoveredUnit` _asbp_unit)
    (if (== (`/Game/_Main/Blueprint/Unit/BP_Unit.TeamIndex` (`local.HoveredUnit`)) (`self.TeamIndex`))
      (if (== (`local.HoveredUnit`) (`self.Focused`))
        (`/Engine/EditorBlueprintResources/StandardMacros.IsValid` (`self.Focused`)
          (:`Is Valid`
            (`self.SetFocusedVisibility` true)))
        (else
          (`/Engine/EditorBlueprintResources/StandardMacros.IsValid` (`self.Focused`)
            (:`Is Valid`
              (`self.SetFocusedVisibility` false))
            (:`Is Not Valid`
              _))
          (set `self.Focused` (`local.HoveredUnit`))))
      (else
        (if true :!label _label
          (`/Engine/EditorBlueprintResources/StandardMacros.IsValid` (`self.Focused`)
            (:`Is Valid`
              (`self.SetFocusedVisibility` false))))))
    (else
      (goto _label))))

(fn `PlayerMovement`
  (params (X :type "Float (double-precision)") (Y :type "Float (double-precision)"))
  (bind _asbp_player (cast `/Game/_Main/Blueprint/Player/BP_Player` (`self.K2_GetPawn`)))
  (bind _arrow (`/Game/_Main/Blueprint/Player/BP_Player.Arrow` _asbp_player))
  (`Pawn.AddMovementInput` _asbp_player (`SceneComponent.GetRightVector` _arrow) (`local.X`) false)
  (`Pawn.AddMovementInput` _asbp_player (`SceneComponent.GetForwardVector` _arrow) (`local.Y`) false))

(fn `ResetArmy`
  (for _array_element (`self.Army`)
    (message `/Game/_Main/Blueprint/Unit/AIController/Interface/BPI_UnitController.Deselected` _array_element))
  (`KismetArrayLibrary.Array_Clear` (`self.Army`))
  (`EnhancedInputSubsystemInterface.RemoveMappingContext` (subsystem `EnhancedInputLocalPlayerSubsystem`) "/Game/_Main/Blueprint/PlayerController/Input/IMC/Order/IMC_Order.IMC_Order" (struct))
  (set `self.bHasArmy` false)
  (set `self.Is Military Army` false))

(fn `RessourceOnClick`
  (returns (bIsSuccessful :type Boolean))
  (bind (_returnvalue _hitactor) (`self.GetActorFromHit` (`|MakeArray` "ObjectTypeQuery6" :!type "EObjectTypeQuery Enum")))
  (`/Engine/EditorBlueprintResources/StandardMacros.IsValid` _hitactor
    (:`Is Valid`
      (if (not (`self.Is Military Army`))
        (`self.SetTargetToUnitInArmy` _hitactor)
        (return true)
        (else
          _)))
    (:`Is Not Valid`
      _))
  (return false))

(fn `SelectBuildingOnClick`
  (bind (_hitresult _returnvalue) (`self.GetHitResultUnderCursorForObjects` (`|MakeArray` "ObjectTypeQuery8" :!type "EObjectTypeQuery Enum")))
  (bind (_bblockinghit _binitialoverlap _time _distance _location _impactpoint _normal _impactnormal _physmat _hitactor) (`GameplayStatics.BreakHitResult` _hitresult))
  (if _returnvalue
    (bind _teamindex (message `/Game/_Main/Blueprint/Interface/BPI_Selectable.GetTeamIndex` _hitactor))
    (if (== _teamindex (`self.TeamIndex`))
      (`/Game/_Main/Blueprint/HUD/BP_HUD.ShowUIBuilding` (cast `/Game/_Main/Blueprint/HUD/BP_HUD` (`self.GetHUD`) :!pure true) (cast `/Game/_Main/Blueprint/Building/BP_Building` _hitactor :!pure true) true))
    (else
      (bind _asbp_hud (cast `/Game/_Main/Blueprint/HUD/BP_HUD` (`self.GetHUD`)))
      (`/Game/_Main/Blueprint/HUD/BP_HUD.ShowUIBuilding` _asbp_hud null false))))

(fn `SelectGroupFromSelectedArmy`
  (locals (SelectUnitGroup :type "Actor Object Reference"))
  (for _array_element (`self.Army`)
    (bind _unitgroup (`/Game/_Main/Blueprint/Unit/AIController/Interface/BPI_UnitController.GetUnitGroup` _array_element))
    (bind _output_get (set `local.SelectUnitGroup` _unitgroup))
    (`/Engine/EditorBlueprintResources/StandardMacros.IsValid` _output_get
      (:`Is Valid`
        (if (`KismetArrayLibrary.Array_IsEmpty` (`self.SelectedUnitGroup`))
          (`KismetArrayLibrary.Array_Add` (`self.SelectedUnitGroup`) (`local.SelectUnitGroup`))
          (bind _group (message `/Game/_Main/Blueprint/UnitGroup/BPI_UnitGroup.GetGroup` (`local.SelectUnitGroup`)))
          (for _array_element_2 _group
            (bind _selectedunit (message `/Game/_Main/Blueprint/Unit/AIController/Interface/BPI_UnitController.Selected` _array_element_2))
            (`KismetArrayLibrary.Array_AddUnique` (`self.Army`) _selectedunit))
          (else
            (for _array_element_3 (`self.SelectedUnitGroup`)
              (set `self.bIsNewGroup` (!= _array_element_3 (`local.SelectUnitGroup`))))
            (if (`self.bIsNewGroup`)
              (`KismetArrayLibrary.Array_Add` (`self.SelectedUnitGroup`) (`local.SelectUnitGroup`))
              (bind _group_2 (message `/Game/_Main/Blueprint/UnitGroup/BPI_UnitGroup.GetGroup` (`local.SelectUnitGroup`)))
              (for _array_element_4 _group_2
                (bind _selectedunit_2 (message `/Game/_Main/Blueprint/Unit/AIController/Interface/BPI_UnitController.Selected` _array_element_4))
                (`KismetArrayLibrary.Array_AddUnique` (`self.Army`) _selectedunit_2))))))))
  (`KismetArrayLibrary.Array_Clear` (`self.SelectedUnitGroup`)))

(fn `SelectUnitOnClick`
  (returns (HasNotSelectedUnit :type Boolean))
  (locals (HitUnit :type "/Game/_Main/Blueprint/Unit/BP_Unit Object Reference") (HittedUnitController :type "AIController Object Reference"))
  (bind _army (`self.Army`))
  (bind (_asbp_unit _bsuccess) (cast `/Game/_Main/Blueprint/Unit/BP_Unit` (`.HitActor` (`self.GetActorFromHit` (`|MakeArray` "ObjectTypeQuery7" :!type "EObjectTypeQuery Enum"))) :!pure true))
  (set `local.HitUnit` _asbp_unit)
  (if _bsuccess
    (set `local.HittedUnitController` (`AIBlueprintHelperLibrary.GetAIController` (`local.HitUnit`)))
    (bind _teamindex (message `/Game/_Main/Blueprint/Interface/BPI_Selectable.GetTeamIndex` (`local.HitUnit`)))
    (if (== _teamindex (`self.TeamIndex`))
      (bind _unitgroup (message `/Game/_Main/Blueprint/Unit/AIController/Interface/BPI_UnitController.GetUnitGroup` (`local.HitUnit`)))
      (`/Engine/EditorBlueprintResources/StandardMacros.IsValid` _unitgroup
        (:`Is Valid`
          (bind (_group _bismilitaryarmy) (message `/Game/_Main/Blueprint/UnitGroup/BPI_UnitGroup.GetGroup` _unitgroup))
          (set `self.Is Military Army` _bismilitaryarmy)
          (for _array_element _group
            (bind _selectedunit (message `/Game/_Main/Blueprint/Unit/AIController/Interface/BPI_UnitController.Selected` _array_element))
            (`KismetArrayLibrary.Array_Add` (`self.Army`) _selectedunit)))
        (:`Is Not Valid`
          (if (`|EnumInequality` (`/Game/_Main/Blueprint/Unit/BP_Unit.Type` (`local.HitUnit`)) "NewEnumerator5")
            (set `self.Is Military Army` true))
          (bind _selectedunit_2 (message `/Game/_Main/Blueprint/Unit/AIController/Interface/BPI_UnitController.Selected` (`local.HittedUnitController`)))
          (`KismetArrayLibrary.Array_AddUnique` (`self.Army`) _selectedunit_2)))
      (`EnhancedInputSubsystemInterface.AddMappingContext` (subsystem `EnhancedInputLocalPlayerSubsystem`) "/Game/_Main/Blueprint/PlayerController/Input/IMC/Order/IMC_Order.IMC_Order" 0 (struct)))
    (else
      (for _array_element_2 _army
        (message `/Game/_Main/Blueprint/Unit/AIController/Interface/BPI_UnitController.Deselected` _array_element_2))
      (`KismetArrayLibrary.Array_Clear` _army)
      (set `self.Is Military Army` false)
      (`EnhancedInputSubsystemInterface.RemoveMappingContext` (subsystem `EnhancedInputLocalPlayerSubsystem`) "/Game/_Main/Blueprint/PlayerController/Input/IMC/Order/IMC_Order.IMC_Order" (struct))
      (return true))))

(fn `SetFocusedVisibility`
  (params (bNewVisibility :type Boolean))
  (bind _unitgroup (message `/Game/_Main/Blueprint/Unit/AIController/Interface/BPI_UnitController.GetUnitGroup` (`AIBlueprintHelperLibrary.GetAIController` (`self.Focused`))))
  (`/Engine/EditorBlueprintResources/StandardMacros.IsValid` _unitgroup
    (:`Is Valid`
      (message `/Game/_Main/Blueprint/UnitGroup/BPI_UnitGroup.FocusAll` _unitgroup (`local.bNewVisibility`)))
    (:`Is Not Valid`
      (`/Game/_Main/Blueprint/Unit/BP_Unit.ToggleFocus` (`self.Focused`) (`local.bNewVisibility`)))))

(fn `SetTargetToUnitInArmy`
  (params (Target :type "Actor Object Reference"))
  (for _array_element (`self.Army`)
    (message `/Game/_Main/Blueprint/Unit/AIController/Interface/BPI_UnitController.CancelAction` _array_element false)
    (message `/Game/_Main/Blueprint/Unit/AIController/Interface/BPI_UnitController.SetTarget` _array_element Target)))

(fn `StartDrawRect`
  (bind (_locationx _locationy) (`self.GetMousePosition`))
  (`/Game/_Main/Blueprint/HUD/BP_HUD.FirstMousePosition` (`self.HUD`) (`KismetMathLibrary.MakeVector2D` _locationx _locationy))
  (`/Game/_Main/Blueprint/HUD/BP_HUD.CanDrawRect` (`self.HUD`) true)
  (`KismetSystemLibrary.K2_PauseTimerHandle` (`self.HoverUnitTimer`)))

(fn `StopDrawRect`
  (`KismetSystemLibrary.K2_UnPauseTimerHandle` (`self.HoverUnitTimer`))
  (`/Game/_Main/Blueprint/HUD/BP_HUD.FirstMousePosition` (`self.HUD`) (0.0 0.0))
  (`/Game/_Main/Blueprint/HUD/BP_HUD.UpdateMousePosition` (`self.HUD`) (0.0 0.0))
  (`/Game/_Main/Blueprint/HUD/BP_HUD.CanDrawRect` (`self.HUD`) false))

(fn `UpdateMousePositionDrawRect`
  (bind (_locationx _locationy) (`self.GetMousePosition`))
  (`/Game/_Main/Blueprint/HUD/BP_HUD.UpdateMousePosition` (`self.HUD`) (`KismetMathLibrary.MakeVector2D` _locationx _locationy)))

(fn `UserConstructionScript`)

(fn `ZoomCamera`
  (params (Zoom :type "Float (double-precision)"))
  (bind (_relativerotation_roll _relativerotation_pitch) (`KismetMathLibrary.BreakRotator` (`SceneComponent.RelativeRotation` (`self.Spring Arm`))))
  (bind (_relativerotation_roll_2 _relativerotation_pitch_2) (`KismetMathLibrary.BreakRotator` (`SceneComponent.RelativeRotation` (`self.Spring Arm`))))
  (set `self.Zoom` Zoom)
  (bind _asbp_player (cast `/Game/_Main/Blueprint/Player/BP_Player` (`GameplayStatics.GetPlayerPawn` 0)))
  (bind _springarm (`/Game/_Main/Blueprint/Player/BP_Player.SpringArm` _asbp_player))
  (set `self.Spring Arm` _springarm)
  (if (== (`SceneComponent.RelativeRotation` _springarm) (struct :`Pitch` -45.0) :`ErrorTolerance` 0.1)
    (if (and (== (`SpringArmComponent.TargetArmLength` (`self.Spring Arm`)) 700.0) (< (`self.Zoom`) 0.0))
      (`SceneComponent.K2_SetRelativeRotation` (`self.Spring Arm`) (`KismetMathLibrary.MakeRotator` 0.0 (`KismetMathLibrary.FClamp` (+ _relativerotation_pitch_2 (* (* (`self.Zoom`) -1.0) 10.0)) -45.0 0.0)) false false)
      (else
        (set `SpringArmComponent.TargetArmLength` (`KismetMathLibrary.FClamp` (+ (* (`self.Zoom`) 100.0) (`SpringArmComponent.TargetArmLength` (`self.Spring Arm`))) 700.0 2200.0) (`self.Spring Arm`))))
    (else
      (`SceneComponent.K2_SetRelativeRotation` (`self.Spring Arm`) (`KismetMathLibrary.MakeRotator` 0.0 (`KismetMathLibrary.FClamp` (+ _relativerotation_pitch (* (* (`self.Zoom`) -1.0) 10.0)) -45.0 0.0)) false false))))