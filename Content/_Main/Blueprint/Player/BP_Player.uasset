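; BP_Player is the player Blueprint, holding a Ressources map of quantities keyed by type.
; AddRessource adds the given quantity to an existing entry, but registers a missing type at zero, discarding the quantity passed in.
; The event graph and construction script contain no active logic.
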(fn `AddRessource`
  (params (Type :type "/Game/_Main/Blueprint/Ressource/E_RessourceType Enum (by ref)") (Quantity :type Integer))
  (bind (_value _returnvalue) (`BlueprintMapLibrary.Map_Find` (`self.Ressources`) (`local.Type`)))
  (if _returnvalue
    (`BlueprintMapLibrary.Map_Add` (`self.Ressources`) (`local.Type`) (+ (`local.Quantity`) _value))
    (else
      (`BlueprintMapLibrary.Map_Add` (`self.Ressources`) (`local.Type`)))))

(fn `UserConstructionScript`)