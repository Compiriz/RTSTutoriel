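; BP_Infantry is the infantry unit Blueprint, handling how the unit reacts to being attacked and takes damage.
; Its Attacked event passes the aggressor to the unit's controller through SetTargetMessage, then switches on the aggressor's unit type.
; Archery attackers deal half damage, while infantry, anti-cavalry and cavalry deal full damage.
; The actor destroys itself once Life reaches zero or below.
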(event `/Game/_Main/Blueprint/Interface/BPI_Selectable.Attacked`
  (params (Aggressor :type "/Game/_Main/Blueprint/Unit/BP_Unit Object Reference") (Damage :type Integer))
  (`/Engine/EditorBlueprintResources/StandardMacros.IsValid` (`self.Aggressor`)
    (:`Is Valid`
      _)
    (:`Is Not Valid`
      (bind _output_get (set `self.Aggressor` Aggressor))))
  (message `/Game/_Main/Blueprint/Unit/AIController/Interface/BPI_UnitController.SetTarget` (`self.GetController`) _output_get)
  (switch `/Game/_Main/Blueprint/Unit/Enum/E_UnitType` (`/Game/_Main/Blueprint/Unit/BP_Unit.Type` (`self.Aggressor`))
    (:`NewEnumerator1`
      (bind _output_get_2 (set `self.Life` (- (`self.Life`) Damage) :!label _label)))
    (:`NewEnumerator2`
      (goto _label))
    (:`NewEnumerator3`
      (bind _output_get_3 (set `self.Life` (- (`self.Life`) (/ Damage 2)))))
    (:`NewEnumerator4`
      (goto _label)))
  (if (or (<= _output_get_2 0) (<= _output_get_3 0))
    (`self.K2_DestroyActor`)))

(fn `UserConstructionScript`
  (`parent.UserConstructionScript`))