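; BP_Harvest is a harvesting unit type that collects resources from a targeted BP_Resource and credits them to a player.
; Its Action is gated by a cooldown, which resets before the target is cast, then calls Extraction using Damage as the amount.
; The returned type and collected quantity go to AddRessource on BP_Player, resolved by a blocking load of the Player soft reference.
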(fn `Action`
  (params (SelectedTarget :type "Object Object Reference"))
  (if (`self.VerifyCooldown`)
    (`self.ResetCooldown`)
    (bind _asbp_resource (cast `/Game/_Main/Blueprint/Ressource/BP_Resource` (`local.SelectedTarget`)))
    (bind (_type _collected) (`/Game/_Main/Blueprint/Ressource/BP_Resource.Extraction` _asbp_resource (`self.Damage`)))
    (bind _returnvalue (`KismetSystemLibrary.LoadAsset_Blocking` (`self.Player`)))
    (bind _asbp_player (cast `/Game/_Main/Blueprint/Player/BP_Player` _returnvalue))
    (`/Game/_Main/Blueprint/Player/BP_Player.AddRessource` _asbp_player _type _collected)))

(fn `UserConstructionScript`
  (`parent.UserConstructionScript`))