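; Military building Blueprint that queues units by class and produces them over time at its spawn point for team 0.
; Queued counts live in a map; each class's build time is read from a briefly spawned, then destroyed instance.
; A looping timer advances progress and spawns units.
; Normal mode decrements counts and refreshes unit button counters, while loop mode keeps them, re-adding finished classes to cycle the queue.
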(fn `AddUnitToList`
  (params (UnitClass :type "/Game/_Main/Blueprint/Unit/BP_Unit Class Reference"))
  (bind (_value _returnvalue) (`BlueprintMapLibrary.Map_Find` (`self.ListSpawnUnit`) (`local.UnitClass`)))
  (if _returnvalue
    (`BlueprintMapLibrary.Map_Add` (`self.ListSpawnUnit`) (`local.UnitClass`) (+ _value 1))
    (else
      (`BlueprintMapLibrary.Map_Add` (`self.ListSpawnUnit`) (`local.UnitClass`) 1)))
  (if (not (`self.bProcessIsActive`))
    (`self.SpawnProcess`)
    (set `self.bProcessIsActive` true))
  (return))

(fn `ProcessIncrementation`
  (if (== (`self.TimeToCreateUnit`) (`self.CreationProcess`))
    (set `self.CreationProcess` 0)
    (`self.SpawnUnit`)
    (if (`self.bIsLoop`)
      (if (== (`BlueprintMapLibrary.Map_Find` (`self.ListSpawnUnit`) (`self.ActualUnitClass`)) (`self.SpawnedUnit`))
        (`KismetSystemLibrary.K2_ClearAndInvalidateTimerHandle` (`self.IncrementationTimer`))
        (`self.SpawnProcess`))
      (else
        (bind _foundwidgets (`WidgetBlueprintLibrary.GetAllWidgetsOfClass` "/Game/_Main/Blueprint/UI/BuildingUI/UIMilitary/Child/UI_UnitButton.UI_UnitButton_C"))
        (for _array_element _foundwidgets
          (bind _unitclass (`/Game/_Main/Blueprint/UI/BuildingUI/UIMilitary/Child/UI_UnitButton.GetUnitClass` _array_element))
          (if (== _unitclass (`self.ActualUnitClass`))
            (`/Game/_Main/Blueprint/UI/BuildingUI/UIMilitary/Child/UI_UnitButton.SetCounter` _array_element (`BlueprintMapLibrary.Map_Find` (`self.ListSpawnUnit`) (`self.ActualUnitClass`)))
            (break)))))
    (else
      (`/Engine/EditorBlueprintResources/StandardMacros.IncrementInt` (`self.CreationProcess`)))))

(fn `SelectClass`
  (returns (SelectedClass :type "/Game/_Main/Blueprint/Unit/BP_Unit Class Reference"))
  (bind (_keypin _valuepin) (`|MapForEach` (`self.ListSpawnUnit`))
    (:`then`
      (if (== _keypin (`self.ActualUnitClass`))
        (if (and (`self.bIsLoop`) (== _valuepin (`self.SpawnedUnit`)))
          (`BlueprintMapLibrary.Map_Remove` (`self.ListSpawnUnit`) (`self.ActualUnitClass`))
          (`BlueprintMapLibrary.Map_Add` (`self.ListSpawnUnit`) (`self.ActualUnitClass`) (`self.SpawnedUnit`))
          (set `self.SpawnedUnit` 0)
          (else
            (return (`self.ActualUnitClass`))))
        (else
          (return _keypin))))))

(fn `SpawnProcess`
  (bind _selectedclass (`self.SelectClass`))
  (bind _output_get (set `self.ActualUnitClass` _selectedclass))
  (bind _returnvalue (`|SpawnActorFromClass` _output_get (`KismetMathLibrary.MakeTransform` (0.0 0.0 -100.0)) "AlwaysSpawn" "MultiplyWithRoot" null null))
  (bind _timetocreate (message `/Game/_Main/Blueprint/Unit/Interface/BPI_Unit.GetTimeTocreate` _returnvalue))
  (set `self.TimeToCreateUnit` _timetocreate)
  (`self.K2_DestroyActor` _returnvalue)
  (bind _returnvalue_2 (`KismetSystemLibrary.K2_SetTimer` null "ProcessIncrementation" 0.1 true))
  (set `self.IncrementationTimer` _returnvalue_2))

(fn `SpawnUnit`
  (bind _incrementationtimer (`self.IncrementationTimer`))
  (bind _returnvalue (- (`BlueprintMapLibrary.Map_Find` (`self.ListSpawnUnit`) (`self.ActualUnitClass`)) 1))
  (bind _returnvalue_2 (`|SpawnActorFromClass` (`self.ActualUnitClass`) (`SceneComponent.K2_GetComponentToWorld` (`self.SpawnPoint`)) "AdjustIfPossibleButAlwaysSpawn" "MultiplyWithRoot" null null))
  (message `/Game/_Main/Blueprint/Unit/Interface/BPI_Unit.SetIdTeam` _returnvalue_2 0)
  (if (`self.bIsLoop`)
    (set `self.SpawnedUnit` (+ (`self.SpawnedUnit`) 1))
    (elif (<= _returnvalue 0)
      (`BlueprintMapLibrary.Map_Remove` (`self.ListSpawnUnit`) (`self.ActualUnitClass`))
      (if (`BlueprintMapLibrary.Map_IsEmpty` (`self.ListSpawnUnit`))
        (`KismetSystemLibrary.K2_ClearAndInvalidateTimerHandle` _incrementationtimer)
        (set `self.bProcessIsActive` false)
        (else
          (`KismetSystemLibrary.K2_ClearAndInvalidateTimerHandle` _incrementationtimer)))
      (else
        (`BlueprintMapLibrary.Map_Add` (`self.ListSpawnUnit`) (`self.ActualUnitClass`) _returnvalue)))))

(fn `UserConstructionScript`
  (`parent.UserConstructionScript`))